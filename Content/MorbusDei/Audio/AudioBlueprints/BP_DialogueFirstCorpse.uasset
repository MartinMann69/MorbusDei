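; BP_DialogueFirstCorpse is a one-shot dialogue trigger, apparently for the first corpse the player encounters.
; On the first actor overlap it creates a WBP_InteractInformationText widget, fills it with DialogueText, adds it to the viewport and sets a Triggered flag.
; When its AudioComponent finishes playing, it removes the widget; the graph itself never starts the audio.
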(event OnAudioFinished(AudioComponent)
  (bind _dialogwidget (Variables|Default|GetDialogWidget))
  (if (Utilities|IsValid _dialogwidget)
    (Widget|RemovefromParent _dialogwidget)))

(event EventBeginPlay)

(event Collision|EventActorBeginOverlap
  (params (OtherActor :type Actor%20Object%20Reference))
  (if (not (Variables|Default|Gettriggered))
    (bind _returnvalue (UserInterface|CreateWidget "/Game/MorbusDei/UI/Widgets/WBP_InteractInformationText.WBP_InteractInformationText_C"))
    (Variables|Default|SetDialogWidget _returnvalue)
    (Default|SetData _returnvalue "" 0 "" (Variables|Default|GetDialogueText))
    (UserInterface|Viewport|AddtoViewport _returnvalue 0)
    (Variables|Default|Settriggered true)))

(fn ConstructionScript)