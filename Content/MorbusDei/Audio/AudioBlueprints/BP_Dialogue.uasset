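; BP_Dialogue is a one-shot dialogue trigger actor that shows dialogue text and freezes player move and look input.
; The first overlap plays a heavy story haptic, locks input and adds a WBP_InteractInformationText widget filled with DialogueText.
; When its AudioComponent finishes, it plays a light haptic and, if the widget is valid, removes it and restores input.
; The graph does not start the audio itself.
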(event OnAudioFinished(AudioComponent)
  (bind _returnvalue (Game|GetPlayerController 0))
  (bind _dialogwidget (Variables|Default|GetDialogWidget))
  (Class|MDHapticBlueprintLibrary|PlayMDHapticEvent "StoryLight")
  (if (Utilities|IsValid _dialogwidget)
    (Widget|RemovefromParent _dialogwidget)
    (Input|SetIgnoreMoveInput _returnvalue false)
    (Input|SetIgnoreLookInput _returnvalue false)))

(event EventBeginPlay)

(event Collision|EventActorBeginOverlap
  (params (OtherActor :type Actor%20Object%20Reference))
  (bind _returnvalue (Game|GetPlayerController 0))
  (if (not (Variables|Default|Gettriggered))
    (Class|MDHapticBlueprintLibrary|PlayMDHapticEvent "StoryHeavy")
    (Input|SetIgnoreMoveInput _returnvalue true)
    (Input|SetIgnoreLookInput _returnvalue true)
    (bind _returnvalue_2 (UserInterface|CreateWidget "/Game/MorbusDei/UI/Widgets/WBP_InteractInformationText.WBP_InteractInformationText_C"))
    (Variables|Default|SetDialogWidget _returnvalue_2)
    (Default|SetData _returnvalue_2 "" 0 "" (Variables|Default|GetDialogueText))
    (UserInterface|Viewport|AddtoViewport _returnvalue_2 0)
    (Variables|Default|Settriggered true)))

(fn ConstructionScript)