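; Blueprint function library giving global access to the game's layered UI system and input focus for a given player controller.
; Layer functions (register, push, pop, clear one, all or all but one) forward to BP_MainHUD through the player's HUD.
; FocusGame and FocusModal forward to BP_MainPlayerController, with modal options for pausing, cursor visibility and UI-only input.
; Failed casts exit silently, so the library holds no UI logic itself.
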(fn RegisterLayer
  (params (OwningPlayer :type Player%20Controller%20Object%20Reference) (LayerName :type Gameplay%20Tag%20Structure :default "(TagName=\"UI.Layer\")") (LayerWidget :type WBP%20Layer%20Object%20Reference))
  (Utilities|IsValid OwningPlayer
    (:Is%20Valid
      (bind _asbp_main_hud (Utilities|Casting|CastToBP_MainHUD (HUD|GetHUD OwningPlayer)))
      (bind _returnvalue (Default|RegisterLayer _asbp_main_hud LayerName LayerWidget))
      (return _returnvalue))))

(fn PushContenttoLayer
  (params (OwningPlayer :type Player%20Controller%20Object%20Reference) (LayerName :type Gameplay%20Tag%20Structure :default "(TagName=\"UI.Layer\")") (WidgetClass :type User%20Widget%20Soft%20Class%20Reference))
  (Utilities|IsValid OwningPlayer
    (:Is%20Valid
      (bind _asbp_main_hud (Utilities|Casting|CastToBP_MainHUD (HUD|GetHUD OwningPlayer)))
      (bind _widget (Default|PushContenttoLayer _asbp_main_hud LayerName WidgetClass))
      (return _widget))))

(fn PopContentfromLayer
  (params (OwningPlayer :type Player%20Controller%20Object%20Reference) (LayerName :type Gameplay%20Tag%20Structure :default "(TagName=\"UI.Layer\")"))
  (Utilities|IsValid OwningPlayer
    (:Is%20Valid
      (bind _asbp_main_hud (Utilities|Casting|CastToBP_MainHUD (HUD|GetHUD OwningPlayer)))
      (Default|PopContentfromLayer _asbp_main_hud LayerName))))

(fn ClearAllLayers
  (params (OwningPlayer :type Player%20Controller%20Object%20Reference))
  (Utilities|IsValid OwningPlayer
    (:Is%20Valid
      (bind _asbp_main_hud (Utilities|Casting|CastToBP_MainHUD (HUD|GetHUD OwningPlayer)))
      (Default|ClearAllLayers _asbp_main_hud))))

(fn ClearLayer
  (params (OwningPlayer :type Player%20Controller%20Object%20Reference) (LayerName :type Gameplay%20Tag%20Structure :default "(TagName=\"UI.Layer\")"))
  (Utilities|IsValid OwningPlayer
    (:Is%20Valid
      (bind _asbp_main_hud (Utilities|Casting|CastToBP_MainHUD (HUD|GetHUD OwningPlayer)))
      (Default|ClearLayer _asbp_main_hud LayerName))))

(fn FocusGame
  (params (OwningPlayer :type Player%20Controller%20Object%20Reference))
  (bind _asbp_main_player_controller (Utilities|Casting|CastToBP_MainPlayerController OwningPlayer))
  (Default|FocusGame _asbp_main_player_controller))

(fn FocusModal
  (params (OwningPlayer :type Player%20Controller%20Object%20Reference) (WidgetToFocus :type Widget%20Object%20Reference) (bPauseGame :type Boolean) (bShowMouseCursor :type Boolean) (bUIOnlyInput :type Boolean))
  (bind _asbp_main_player_controller (Utilities|Casting|CastToBP_MainPlayerController OwningPlayer))
  (Default|FocusModal _asbp_main_player_controller WidgetToFocus bPauseGame bShowMouseCursor bUIOnlyInput))

(fn ClearAllLayerExcept
  (params (OwningPlayer :type Player%20Controller%20Object%20Reference) (ExceptionLayerName :type Gameplay%20Tag%20Structure :default "(TagName=\"UI.Layer\")"))
  (Utilities|IsValid OwningPlayer
    (:Is%20Valid
      (bind _asbp_main_hud (Utilities|Casting|CastToBP_MainHUD (HUD|GetHUD OwningPlayer)))
      (Default|ClearAllLayersExcept _asbp_main_hud ExceptionLayerName))))