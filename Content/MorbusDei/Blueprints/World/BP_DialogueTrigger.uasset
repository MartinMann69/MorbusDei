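; BP_DialogueTrigger is a trigger volume that shows dialogue text and plays a sound when the player walks into it.
; On overlap with BP_PlayerCharacter it creates a WBP_InteractInformationText widget, fills it with DialogueText and adds it to the viewport.
; It then spawns an actor of AudioZoneClass and calls PlayZoneSound on it.
; With TriggerOnlyOnce set, it disables the box collision afterwards so it does not fire again.
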(event EventBeginPlay)

(event EventTick
  (params (DeltaSeconds :type Float%20%28single-precision%29)))

(event Collision|EventActorBeginOverlap
  (params (OtherActor :type Actor%20Object%20Reference))
  (Utilities|Casting|CastToBP_PlayerCharacter OtherActor)
  (bind _returnvalue (UserInterface|CreateWidget "/Game/MorbusDei/UI/Widgets/WBP_InteractInformationText.WBP_InteractInformationText_C"))
  (Default|SetData _returnvalue "" 0 "" (Variables|Default|GetDialogueText))
  (UserInterface|Viewport|AddtoViewport _returnvalue 0)
  (bind _returnvalue_2 (Game|SpawnActorfromClass (Variables|Default|GetAudioZoneClass) (Math|Transform|MakeTransform "0, 0, 0" "0, 0, 0" "1.000000,1.000000,1.000000") "Undefined" "MultiplyWithRoot" 0 0))
  (Class|MDAudioZone|PlayZoneSound _returnvalue_2)
  (if (Variables|Default|GetTriggerOnlyOnce)
    (Collision|SetCollisionEnabled (Variables|Default|GetBox) "NoCollision")))

(fn ConstructionScript)