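; BP_Mirror is an interactable mirror that shows an information widget with text, an image and dialogue when used.
; Interact runs the parent behavior, then waits for a voiceover delay that follows the interaction sound.
; It then creates a WBP_InteractInformationText widget, fills it from its info text, image and dialogue variables, and adds it to the viewport.
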(event EventBeginPlay)

(event Collision|EventActorBeginOverlap
  (params (OtherActor :type Actor%20Object%20Reference)))

(event EventTick
  (params (DeltaSeconds :type Float%20%28single-precision%29)))

(event EventInteract
  (params (Interactor :type Pawn%20Object%20Reference))
  (|CallParentFunction Interactor)
  (Utilities|FlowControl|Delay (Variables|Default|GetVoiceoverDelayAfterInteractionSound))
  (bind _returnvalue (UserInterface|CreateWidget "/Game/MorbusDei/UI/Widgets/WBP_InteractInformationText.WBP_InteractInformationText_C"))
  (bind _output_get (Variables|MD|SetWidgetRef _returnvalue))
  (Default|SetData _output_get (Variables|MD|GetInfoText) (Variables|MD|GetInfoImage) (Variables|MD|GetInfoText_2) (Variables|MD|GetDialogueText))
  (UserInterface|Viewport|AddtoViewport (Variables|MD|GetWidgetRef) 0))

(fn ConstructionScript)