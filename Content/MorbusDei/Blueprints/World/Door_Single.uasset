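; Single swinging door Blueprint in the world that opens once when interacted with and cannot be closed again.
; BeginPlay caches the closed pivot rotation, derives the open one from a yaw angle, and configures the timeline with an assignable curve and a play rate from the open duration.
; Interact passes a DoOnce, calls the parent, disables further interaction, then plays the timeline to lerp the pivot between both rotations by shortest path.
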(event EventInteract
  (params (Interactor :type Pawn%20Object%20Reference))
  (Utilities|FlowControl|DoOnce false
    (:Completed
      (|CallParentFunction Interactor)
      (Variables|Default|SetbCanInteract false)
      (bind _alpha (Timeline|TL_Door PlayFromStart)
        (:Update
          (Transformation|SetRelativeRotation (Variables|Default|GetDoorPivot) (Math|Rotator|Lerp(Rotator) (Variables|Default|GetClosedRotation) (Variables|Default|GetOpenRotation) _alpha true) false false))))))

(event EventBeginPlay
  (|CallParentFunction)
  (Class|TimelineComponent|SetFloatCurve (Variables|Default|GetTL_Door) (Variables|MD|Interaction|Door|GetDoorCurve) "Alpha")
  (Components|Timeline|SetPlayRate (Variables|Default|GetTL_Door) (/ 1.0 (Variables|MD|Interaction|Door|GetOpenDuration)))
  (Variables|Default|SetClosedRotation (Variables|/Script/Engine.SceneComponent|GetRelativeRotation (Variables|Default|GetDoorPivot)))
  (Variables|Default|SetOpenRotation (Math|Rotator|CombineRotators (Variables|Default|GetClosedRotation) (Math|Rotator|MakeRotator 0.0 0.0 (Variables|MD|Interaction|Door|GetOpenAngle)))))

(fn ConstructionScript)