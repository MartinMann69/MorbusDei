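; BP_EndGame is an interactable that ends the game by playing an outro and credits, then opening a level.
; Interacting disables further interaction and plays a placeholder intro cutscene as the outro through BP_VideoManager.
; Video-finished bindings chain the outro into the credits video, then into opening LevelToOpen.
; Both videos stop existing sounds and do not restore player control; no binding is removed between them.
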(event Custom|OutroVideoFinished
  (params (VideoId :type Name))
  (EventDispatchers|BindEventtoOnVideoFinished (stale EventInteract _returnvalue) (delegate Custom|CreditsVideoFinished))
  (Class|MDVideoManager|PlayVideo (stale EventInteract _returnvalue) "/Game/Movies/credits_v1_75sec.credits_v1_75sec" "None" true false true))

(event Custom|CreditsVideoFinished
  (params (VideoId :type Name))
  (Game|OpenLevel(byObjectReference) (Utilities|Struct|BreakSoftWorldReference (Variables|Default|GetLevelToOpen))))

(event EventInteract
  (params (Interactor :type Pawn%20Object%20Reference))
  (|CallParentFunction Interactor)
  (Variables|Default|SetbCanInteract false)
  (bind _returnvalue (Actor|GetActorOfClass "/Game/MorbusDei/Blueprints/Video/BP_VideoManager.BP_VideoManager_C"))
  (EventDispatchers|BindEventtoOnVideoFinished _returnvalue (delegate Custom|OutroVideoFinished))
  (Class|MDVideoManager|PlayVideo _returnvalue "/Game/Movies/Intro_Cutscene_Placeholder_Version.Intro_Cutscene_Placeholder_Version" "None" true false true))

(fn ConstructionScript)