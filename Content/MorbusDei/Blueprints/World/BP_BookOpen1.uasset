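; Interactable open book that shows an information overlay with text, image and dialogue while freezing player movement and look.
; Interact runs the parent logic, locks input, then creates and fills WBP_InteractInformationText after a voiceover delay.
; The spawned audio zone's finish event removes the widget and restores input.
; Re-interaction is blocked while the widget is in the viewport and until shortly after its closed event fires.
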(event Custom|OnWidgetClosed
  (Utilities|FlowControl|Delay 0.2)
  (Variables|Default|SetbCanInteract true))

(event EventBeginPlay)

(event Collision|EventActorBeginOverlap
  (params (OtherActor :type Actor%20Object%20Reference)))

(event EventTick
  (params (DeltaSeconds :type Float%20%28single-precision%29)))

(event EventInteract
  (params (Interactor :type Pawn%20Object%20Reference))
  (bind _returnvalue (Game|GetPlayerController 0))
  (|CallParentFunction Interactor)
  (Variables|Default|SetbCanInteract false)
  (Input|SetIgnoreMoveInput _returnvalue true)
  (Input|SetIgnoreLookInput _returnvalue true)
  (Utilities|FlowControl|Delay (Variables|Default|GetVoiceoverDelayAfterInteractionSound))
  (bind _returnvalue_2 (UserInterface|CreateWidget "/Game/MorbusDei/UI/Widgets/WBP_InteractInformationText.WBP_InteractInformationText_C"))
  (EventDispatchers|BindEventtoOnWidgetClosed _returnvalue_2 (delegate Custom|OnWidgetClosed))
  (bind _output_get (Variables|MD|SetWidgetRef _returnvalue_2))
  (Default|SetData _output_get (Variables|MD|GetInfoText) (Variables|MD|GetInfoImage) (Variables|MD|GetInfoText_2) (Variables|MD|GetDialogueText))
  (UserInterface|Viewport|AddtoViewport (Variables|MD|GetWidgetRef) 0))

(event EventOnSpawnedAudioZoneFinished
  (bind _returnvalue (Game|GetPlayerController 0))
  (Widget|RemovefromParent (Variables|MD|GetWidgetRef))
  (Input|SetIgnoreMoveInput _returnvalue false)
  (Input|SetIgnoreLookInput _returnvalue false))

(fn ConstructionScript)

(fn CanInteract
  (bind _widgetref (Variables|MD|GetWidgetRef))
  (bind _bcaninteract (Variables|Default|GetbCanInteract))
  (Utilities|IsValid _widgetref
    (:Is%20Valid
      (return (and (not (UserInterface|Viewport|IsinViewport _widgetref)) _bcaninteract)))
    (:Is%20Not%20Valid
      (return _bcaninteract))))