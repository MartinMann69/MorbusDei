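; BP_DonationCertificate is an interactable donation certificate that shows information text and an optional follow-up reaction.
; Interact runs the parent logic, disables interaction, ignores move and look input, then after a delay opens WBP_InteractInformationText.
; On close, any ReactionText opens a second widget and spawns an audio zone to play sound.
; Interaction re-enables after the last close; this graph's input-restore nodes are unconnected.
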(event Custom|OnWidgetClosed
  (if (Utilities|Text|TextIsEmpty (Variables|MD|GetReactionText))
    (Utilities|FlowControl|Delay 0.2)
    (Variables|Default|SetbCanInteract true)
    (else
      (bind _returnvalue (UserInterface|CreateWidget "/Game/MorbusDei/UI/Widgets/WBP_InteractInformationText.WBP_InteractInformationText_C"))
      (bind _output_get (Variables|MD|SetWidgetRef _returnvalue))
      (Default|SetData _output_get "" 0 "" (Variables|MD|GetReactionText))
      (UserInterface|Viewport|AddtoViewport _output_get 0)
      (EventDispatchers|BindEventtoOnWidgetClosed _output_get (delegate Custom|OnDialogueClosed))
      (Utilities|FlowControl|DelayUntilNextTick)
      (bind _returnvalue_2 (Game|SpawnActorfromClass (Variables|MD|Audio|GetAudio%20Zone%20Class2) (Transformation|GetActorTransform) "AlwaysSpawn" "MultiplyWithRoot" 0 0))
      (Class|MDAudioZone|PlayZoneSound _returnvalue_2))))

(event Custom|OnDialogueClosed
  (Utilities|FlowControl|Delay 0.2)
  (Variables|Default|SetbCanInteract true))

(event EventBeginPlay)

(event Collision|EventActorBeginOverlap
  (params (OtherActor :type Actor%20Object%20Reference)))

(event EventTick
  (params (DeltaSeconds :type Float%20%28single-precision%29)))

(event EventInteract
  (params (Interactor :type Pawn%20Object%20Reference))
  (bind _returnvalue (Game|GetPlayerController 0))
  (|CallParentFunction Interactor)
  (Variables|Default|SetbCanInteract false)
  (Input|SetIgnoreMoveInput _returnvalue true)
  (Input|SetIgnoreLookInput _returnvalue true)
  (Utilities|FlowControl|Delay (Variables|Default|GetVoiceoverDelayAfterInteractionSound))
  (bind _returnvalue_2 (UserInterface|CreateWidget "/Game/MorbusDei/UI/Widgets/WBP_InteractInformationText.WBP_InteractInformationText_C"))
  (EventDispatchers|BindEventtoOnWidgetClosed _returnvalue_2 (delegate Custom|OnWidgetClosed))
  (bind _output_get (Variables|MD|SetWidgetRef _returnvalue_2))
  (Default|SetData _output_get (Variables|MD|GetInfoText) (Variables|MD|GetInfoImage) (Variables|MD|GetInfoText_2) (Variables|MD|GetDialogueText) "" (Variables|MD|GetSinglePageText))
  (UserInterface|Viewport|AddtoViewport (Variables|MD|GetWidgetRef) 0))

(fn ConstructionScript)