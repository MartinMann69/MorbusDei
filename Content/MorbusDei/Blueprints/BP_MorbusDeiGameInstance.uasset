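; Game instance for MorbusDei that owns the player's audio volume settings and applies them when the game starts.
; On init it activates the volume sound mix, then loads the audio settings save from its slot, creating and saving a new one if none exists.
; It overrides the Master, Music and SFX sound classes, multiplying Music and SFX by master volume manually instead of propagating to child classes.
; A separate function writes current settings back to the slot.
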(event EventInit
  (Class|GameplayStatics|SetBaseSoundMix "/Game/MorbusDei/Audio/SoundClasses/SM_VolumeSettings.SM_VolumeSettings")
  (Audio|PushSoundMixModifier "/Game/MorbusDei/Audio/SoundClasses/SM_VolumeSettings.SM_VolumeSettings")
  (CallFunction|LoadAudioSettings))

(fn LoadAudioSettings
  (bind _slot_name (Variables|Default|GetSlot%20Name))
  (bind _returnvalue (SaveGame|DoesSaveGameExist _slot_name))
  (if _returnvalue
    (bind _returnvalue_2 (SaveGame|LoadGamefromSlot _slot_name))
    (bind _asbp_audio_settings_save (Utilities|Casting|CastToBP_AudioSettingsSave _returnvalue_2))
    (Variables|Default|SetAudioSettingsSave _asbp_audio_settings_save)
    (else
      (bind _returnvalue_3 (SaveGame|CreateSaveGameObject "/Game/MorbusDei/Blueprints/BP_AudioSettingsSave.BP_AudioSettingsSave_C"))
      (bind _output_get (Variables|Default|SetAudioSettingsSave _returnvalue_3))
      (SaveGame|SaveGametoSlot _output_get _slot_name)))
  (CallFunction|ApplyAudioSettings))

(fn ApplyAudioSettings
  (bind _volumesettings (Variables|Default|GetVolumeSettings))
  (bind _audiosettingssave (Variables|Default|GetAudioSettingsSave))
  (bind _mastervolume (Variables|/Game/MorbusDei/Blueprints/BP_AudioSettingsSave.BP_AudioSettingsSave_C|GetMasterVolume _audiosettingssave))
  (Audio|SetSoundMixClassOverride _volumesettings "/Game/MorbusDei/Audio/SoundClasses/SC_Master.SC_Master" _mastervolume 1.0 0.1 false)
  (Audio|SetSoundMixClassOverride _volumesettings "/Game/MorbusDei/Audio/SoundClasses/SC_Music.SC_Music" (* _mastervolume (Variables|/Game/MorbusDei/Blueprints/BP_AudioSettingsSave.BP_AudioSettingsSave_C|GetMusicVolume _audiosettingssave)) 1.0 0.1 false)
  (Audio|SetSoundMixClassOverride _volumesettings "/Game/MorbusDei/Audio/SoundClasses/SC_SFX.SC_SFX" (* _mastervolume (Variables|/Game/MorbusDei/Blueprints/BP_AudioSettingsSave.BP_AudioSettingsSave_C|GetSFXVolume _audiosettingssave)) 1.0 0.1 false))

(fn SaveAudioSettings
  (SaveGame|SaveGametoSlot (Variables|Default|GetAudioSettingsSave) (Variables|Default|GetSlot%20Name)))